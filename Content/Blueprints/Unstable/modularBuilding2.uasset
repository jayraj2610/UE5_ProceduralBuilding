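; Work-in-progress modular building Blueprint that assembles corner and wall pieces from configurable meshes in the Construction Script.
; It assigns meshes to components (Wall and WallRoof receive upper and middle meshes, seemingly swapped), then adds Corner instances per height step at one fixed offset, ignoring the index.
; Uncalled helpers spawn individual lower, middle or upper mesh components, applying location and rotation offsets to corners.
; Other offset helpers are unfinished.
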(event EventBeginPlay)

(fn ConstructionScript
  (Utilities|FlowControl|Sequence
    (:then_0
      (CallFunction|SetMeshVariables))
    (:then_1
      (Variables|Default|SetStartLocation (Transformation|GetRelativeTransform (Variables|Default|GetDefaultSceneRoot))))
    (:then_2
      (for _index (range 1 (Variables|BuildingSize|GetNumOfMiddlePieceHeight))
        (Components|InstancedStaticMesh|AddInstance (Variables|Default|GetCorner) (Math|Transform|MakeTransform (+ (Math|Vector|MakeVector (Variables|AssetSize|GetCornerX_Width) 0.0 0.0) (.location (Variables|Default|GetStartLocation))) "0, 0, 0" "1.000000,1.000000,1.000000") false)))))

(fn HandleTypeandSpawnMeshComp
  (params (Transform :type Transform) (isCorner :type Boolean) (CounterIndex :type Integer) (First%20timeGenratingCorner :type Boolean))
  (bind (_location _rotation _scale) (Math|Transform|BreakTransform Transform))
  (bind _cornerrotationoffset (Variables|Offset|GetCornerRotationOffset))
  (bind _cornerlocationoffset (Variables|Offset|GetCornerLocationOffset))
  (bind _returnvalue (Math|Rotator|CombineRotators _rotation _cornerrotationoffset))
  (bind _returnvalue_2 (+ _location _cornerlocationoffset))
  (bind _returnvalue_3 (Math|Transform|MakeTransform _returnvalue_2 _returnvalue _scale))
  (if isCorner
    (Utilities|Position CounterIndex
      (:Lower
        (bind _meshcompref (Utilities|SpawnMesh _returnvalue_3 (Variables|StaticMesh|GetLowerCornerMesh)))
        (return _meshcompref))
      (:Mid
        (bind _meshcompref_2 (Utilities|SpawnMesh _returnvalue_3 (Variables|StaticMesh|GetCornerMesh)))
        (return _meshcompref_2))
      (:Upper
        (bind _meshcompref_3 (Utilities|SpawnMesh _returnvalue_3 (Variables|StaticMesh|GetUpperCornerMesh)))
        (return _meshcompref_3)))
    (else
      (Utilities|Position CounterIndex
        (:Lower
          (bind _meshcompref_4 (Utilities|SpawnMesh Transform (Variables|StaticMesh|GetLowerMidTileMesh)))
          (return _meshcompref_4))
        (:Mid
          (bind _meshcompref_5 (Utilities|SpawnMesh Transform (Variables|StaticMesh|GetMidTileMesh)))
          (return _meshcompref_5))
        (:Upper
          (bind _meshcompref_6 (Utilities|SpawnMesh Transform (Variables|StaticMesh|GetUpperMidTileMesh)))
          (return _meshcompref_6))))))

(fn SetMeshVariables
  ;[1 1 1] corner
  (Components|StaticMesh|SetStaticMesh (Variables|Default|GetCorner) (Variables|StaticMesh|GetCornerMesh))
  (Components|StaticMesh|SetStaticMesh (Variables|Default|GetCornerBottom) (Variables|StaticMesh|GetLowerCornerMesh))
  (Components|StaticMesh|SetStaticMesh (Variables|Default|GetCornerRoof) (Variables|StaticMesh|GetUpperCornerMesh))
  ;[1 1 1] wall
  (Components|StaticMesh|SetStaticMesh (Variables|Default|GetWallBottom) (Variables|StaticMesh|GetLowerMidTileMesh))
  (Components|StaticMesh|SetStaticMesh (Variables|Default|GetWall) (Variables|StaticMesh|GetUpperMidTileMesh))
  (Components|StaticMesh|SetStaticMesh (Variables|Default|GetWallRoof) (Variables|StaticMesh|GetMidTileMesh)))
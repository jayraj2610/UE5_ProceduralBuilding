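; Procedural modular building actor whose construction script assembles a rectangular shell of static mesh components, with optional roof, floor and corner pillars.
; Four chained wall loops call HandleTypeAndSpawnMeshComp, choosing door, window or lower/mid/upper meshes by side and grid index.
; Windows follow location arrays or an alternating pattern; saved row ends position pillars and can be hidden or destroyed.
; BakeMesh copies child mesh transforms into a spawned LightWeightInstanceStaticMeshManager's single instanced component.
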(event EventBeginPlay)

(fn ConstructionScript
  (bind _defaultsceneroot (Variables|Default|GetDefaultSceneRoot))
  (bind _wallx_width (Variables|AssetSize|Wall|GetWallX_Width))
  (bind _wallx_width_2 (Variables|AssetSize|Wall|GetWallX_Width))
  (bind _wallx_width_3 (Variables|AssetSize|Wall|GetWallX_Width))
  (bind _returnvalue (Transformation|GetWorldTransform _defaultsceneroot))
  (Utilities|FlowControl|Sequence
    (:then_0
      (Variables|Default|SetStartLocation (Math|Transform|MakeTransform (.location _returnvalue) (.rotation _returnvalue) (.scale _returnvalue))))
    (:then_1
      (for (_array_element _array_index) (Variables|Window|GetWindowLocationsArray_X)
        (Utilities|Array|SetArrayElem (Variables|Window|GetTempWindowLocation_X) _array_index _array_element true)))
    (:then_2
      (for (_array_element_2 _array_index_2) (Variables|Window|GetWindowLocationsArray_Y)
        (Utilities|Array|SetArrayElem (Variables|Window|GetTempWindowLocation_Y) _array_index_2 _array_element_2 true)))
    (:then_3
      ;[1 1 1] Front X+
      (for _index (range 0 (- (Variables|BuildingSize|GetNumOfWallPieceHeight) 1))
        (for _index_2 (range 0 (- (Variables|BuildingSize|GetNumOfWallPieceRow) 1))
          (bind _meshcompref (CallFunction|HandleTypeandSpawnMeshComp (Math|Transform|MakeTransform (+ (Math|Vector|MakeVector (* _index_2 (Variables|AssetSize|Wall|GetWallX_Width)) 0.0 (* _index (Variables|AssetSize|Wall|GetWallZ_Height))) (.location (Variables|Default|GetStartLocation))) "0, 0, 0" "1.000000,1.000000,1.000000") _index _index_2 "NewEnumerator0" "NewEnumerator0"))
          (bind _output_get (Variables|Default|SetLastTile _meshcompref))
          (Utilities|SaveFirstandLastWallOfRow _output_get _index_2 true))
        (Utilities|Array|Add (Variables|Default|GetLastTileArray) (Variables|Default|GetLastTile))
        (Utilities|Array|Add (Variables|Pillar|GetPillar_1_Transform) (Transformation|GetRelativeTransform (Variables|Default|GetLastTile))))
      ;[1 1 1] Right Y-
      (for _index_3 (range 0 (- (Variables|BuildingSize|GetNumOfWallPieceHeight) 1))
        (for _index_4 (range 0 (- (Variables|BuildingSize|GetNumOfWallPieceLength) 1))
          (bind _meshcompref_2 (CallFunction|HandleTypeandSpawnMeshComp (Math|Transform|MakeTransform (select (== _index_4 0) (+ (Math|Vector|MakeVector _wallx_width_3 0.0 0.0) (.location (Transformation|GetRelativeTransform (Utilities|Array|Get(acopy) (Variables|Default|GetLastTileArray) _index_3)))) (+ (.location (Transformation|GetRelativeTransform (Variables|Default|GetLastTile))) (Math|Vector|MakeVector 0.0 (* _wallx_width_3 -1.0) 0.0))) (Math|Rotator|CombineRotators (.rotation (Transformation|GetRelativeTransform (Utilities|Array|Get(acopy) (Variables|Default|GetLastTileArray) _index_3))) "0.000000,-90.000000,0.000000") "1.000000,1.000000,1.000000") _index_3 _index_4 "NewEnumerator3" "NewEnumerator0"))
          (bind _output_get_2 (Variables|Default|SetLastTile _meshcompref_2))
          (Utilities|SaveFirstandLastWallOfRow _output_get_2 _index_4 false))
        (Utilities|Array|Add (Variables|Default|GetLastTileArray2) (Variables|Default|GetLastTile))
        (Utilities|Array|Add (Variables|Pillar|GetPillar_2_Transform) (Transformation|GetRelativeTransform (Variables|Default|GetLastTile))))
      (Utilities|Array|Clear (Variables|Default|GetLastTileArray))
      ;[1 1 1] Back X-
      (for _index_5 (range 0 (- (Variables|BuildingSize|GetNumOfWallPieceHeight) 1))
        (for _index_6 (range 0 (- (Variables|BuildingSize|GetNumOfWallPieceRow) 1))
          (bind _meshcompref_3 (CallFunction|HandleTypeandSpawnMeshComp (Math|Transform|MakeTransform (select (== _index_6 0) (+ (Math|Vector|MakeVector 0.0 (* _wallx_width -1.0) 0.0) (.location (Transformation|GetRelativeTransform (Utilities|Array|Get(acopy) (Variables|Default|GetLastTileArray2) _index_5)))) (+ (.location (Transformation|GetRelativeTransform (Variables|Default|GetLastTile))) (Math|Vector|MakeVector (* _wallx_width -1.0) 0.0 0.0))) (Math|Rotator|CombineRotators (.rotation (Transformation|GetRelativeTransform (Utilities|Array|Get(acopy) (Variables|Default|GetLastTileArray2) _index_5))) "0.000000,-90.000000,0.000000") "1.000000,1.000000,1.000000") _index_5 _index_6 "NewEnumerator1" "NewEnumerator0"))
          (bind _output_get_3 (Variables|Default|SetLastTile _meshcompref_3))
          (Utilities|SaveFirstandLastWallOfRow _output_get_3 _index_6 true))
        (Utilities|Array|Add (Variables|Default|GetLastTileArray) (Variables|Default|GetLastTile))
        (Utilities|Array|Add (Variables|Pillar|GetPillar_3_Transform) (Transformation|GetRelativeTransform (Variables|Default|GetLastTile))))
      (Utilities|Array|Clear (Variables|Default|GetLastTileArray2))
      ;[1 1 1] Left Y+
      (for _index_7 (range 0 (- (Variables|BuildingSize|GetNumOfWallPieceHeight) 1))
        (for _index_8 (range 0 (- (Variables|BuildingSize|GetNumOfWallPieceLength) 1))
          (bind _meshcompref_4 (CallFunction|HandleTypeandSpawnMeshComp (Math|Transform|MakeTransform (select (== _index_8 0) (+ (Math|Vector|MakeVector (* _wallx_width_2 -1.0) 0.0 0.0) (.location (Transformation|GetRelativeTransform (Utilities|Array|Get(acopy) (Variables|Default|GetLastTileArray) _index_7)))) (+ (.location (Transformation|GetRelativeTransform (Variables|Default|GetLastTile))) (Math|Vector|MakeVector 0.0 _wallx_width_2 0.0))) (Math|Rotator|CombineRotators (.rotation (Transformation|GetRelativeTransform (Utilities|Array|Get(acopy) (Variables|Default|GetLastTileArray) _index_7))) "0.000000,-90.000000,0.000000") "1.000000,1.000000,1.000000") _index_7 _index_8 "NewEnumerator2" "NewEnumerator0"))
          (bind _output_get_4 (Variables|Default|SetLastTile _meshcompref_4))
          (Utilities|SaveFirstandLastWallOfRow _output_get_4 _index_8 false))
        (Utilities|Array|Add (Variables|Default|GetLastTileArray2) (Variables|Default|GetLastTile))
        (Utilities|Array|Add (Variables|Pillar|GetPillar_4_Transform) (Transformation|GetRelativeTransform (Variables|Default|GetLastTile))))
      (Utilities|Array|Clear (Variables|Default|GetLastTileArray))
      (Utilities|FlowControl|Sequence
        (:then_0
          (Utilities|FlowControl|Sequence
            (:then_0
              (if (Variables|Roof|GetGenerate%20Roof)
                ;[1 1 1] Roof
                (for _index_9 (range 0 (- (Variables|BuildingSize|GetNumOfWallPieceLength) 1))
                  (for _index_10 (range 0 (- (Variables|BuildingSize|GetNumOfWallPieceRow) 1))
                    (Utilities|SpawnMesh (Math|Transform|MakeTransform (+ (.location (Variables|Default|GetStartLocation)) (Math|Vector|MakeVector (* _index_10 (Variables|AssetSize|Wall|GetWallX_Width)) (* _index_9 (Variables|AssetSize|Wall|GetWallZ_Height) -1.0) (+ (* (Variables|AssetSize|Wall|GetWallZ_Height) (Variables|BuildingSize|GetNumOfWallPieceHeight)) (Variables|Roof|GetRoofZOffset)))) (Math|Rotator|CombineRotators (Math|Rotator|CombineRotators (.rotation (Variables|Default|GetStartLocation)) "0.000000,0.000000,180.000000") (Variables|Roof|GetRoofRotationOffset)) (Variables|Roof|GetRoofScale)) (Variables|StaticMesh|GetRoofMesh))))))
            (:then_1
              (if (Variables|Floor|GetGenerate%20Floor)
                ;[1 1 1] Floor
                (for _index_11 (range 0 (- (Variables|BuildingSize|GetNumOfWallPieceLength) 1))
                  (for _index_12 (range 0 (- (Variables|BuildingSize|GetNumOfWallPieceRow) 1))
                    (Utilities|SpawnMesh (Math|Transform|MakeTransform (+ (.location (Variables|Default|GetStartLocation)) (Math|Vector|MakeVector (* _index_12 (Variables|AssetSize|Wall|GetWallX_Width)) (* _index_11 (Variables|AssetSize|Wall|GetWallZ_Height) -1.0) (Variables|Floor|GetFloorZOffset))) (Math|Rotator|CombineRotators (Math|Rotator|CombineRotators (.rotation (Variables|Default|GetStartLocation)) "0.000000,0.000000,180.000000") (Variables|Floor|GetFloorRotationOffset)) (Variables|Floor|GetFloorScale)) (Variables|StaticMesh|GetFloorMesh))))))))
        (:then_1
          (if (Variables|Pillar|GetGenerate%20Pillar)
            (Utilities|FlowControl|Sequence
              (:then_0
                ;[1 1 1] Pillar1 Front
                (for _index_13 (range 0 (- (Variables|BuildingSize|GetNumOfWallPieceHeight) 1))
                  (CallFunction|HandleTypeandSpawnMeshComp (Math|Transform|MakeTransform (+ (.location (Utilities|Array|Get(acopy) (Variables|Pillar|GetPillar_1_Transform) _index_13)) (Math|Vector|MakeVector 0.0 0.0 0.0)) (.rotation (Utilities|Array|Get(acopy) (Variables|Pillar|GetPillar_1_Transform) _index_13)) (Variables|Pillar|Mid|GetPillarScale)) _index_13 0 "NewEnumerator0" "NewEnumerator4")))
              (:then_1
                ;[1 1 1] Pillar2 Right
                (for _index_14 (range 0 (- (Variables|BuildingSize|GetNumOfWallPieceHeight) 1))
                  (CallFunction|HandleTypeandSpawnMeshComp (Math|Transform|MakeTransform (+ (.location (Utilities|Array|Get(acopy) (Variables|Pillar|GetPillar_2_Transform) _index_14)) (Math|Vector|MakeVector 0.0 0.0 0.0)) (.rotation (Utilities|Array|Get(acopy) (Variables|Pillar|GetPillar_2_Transform) _index_14)) (Variables|Pillar|Mid|GetPillarScale)) _index_14 0 "NewEnumerator3" "NewEnumerator4")))
              (:then_2
                ;[1 1 1] Pillar3 Back
                (for _index_15 (range 0 (- (Variables|BuildingSize|GetNumOfWallPieceHeight) 1))
                  (CallFunction|HandleTypeandSpawnMeshComp (Math|Transform|MakeTransform (+ (.location (Utilities|Array|Get(acopy) (Variables|Pillar|GetPillar_3_Transform) _index_15)) (Math|Vector|MakeVector 0.0 0.0 0.0)) (.rotation (Utilities|Array|Get(acopy) (Variables|Pillar|GetPillar_3_Transform) _index_15)) (Variables|Pillar|Mid|GetPillarScale)) _index_15 0 "NewEnumerator1" "NewEnumerator4")))
              (:then_3
                ;[1 1 1] Pillar4 Left
                (for _index_16 (range 0 (- (Variables|BuildingSize|GetNumOfWallPieceHeight) 1))
                  (CallFunction|HandleTypeandSpawnMeshComp (Math|Transform|MakeTransform (+ (.location (Utilities|Array|Get(acopy) (Variables|Pillar|GetPillar_4_Transform) _index_16)) (Math|Vector|MakeVector 0.0 0.0 0.0)) (.rotation (Utilities|Array|Get(acopy) (Variables|Pillar|GetPillar_4_Transform) _index_16)) (Variables|Pillar|Mid|GetPillarScale)) _index_16 0 "NewEnumerator2" "NewEnumerator4"))))))
        (:then_2
          (Utilities|HandleFirstandLastWallOFRows))))))

(fn HandleTypeandSpawnMeshComp
  (params (Transform :type Transform) (Height_Index :type Integer) (Row_Index :type Integer) (PillarDirection :type E_Direction%20Enum :default "NewEnumerator0") (Type :type E_Type%20Enum :default "NewEnumerator0"))
  (bind (_location _rotation) (Math|Transform|BreakTransform Transform))
  (bind (_location_2 _rotation_2) (Math|Transform|BreakTransform Transform))
  (bind (_location_3 _rotation_3 _scale) (Math|Transform|BreakTransform Transform))
  (bind _returnvalue (== 0 Height_Index))
  (bind _returnvalue_2 (== Height_Index 0))
  (bind _door_rotationoffset (Variables|Door|GetDoor_RotationOffset))
  (bind _doorlocationoffset (Variables|Door|GetDoorLocationOffset))
  (bind _doorx_location_innoofwalls (Variables|Door|GetDoorX_Location_inNoOfWalls))
  (bind _windowlocationoffset (Variables|Window|GetWindowLocationOffset))
  (bind _doory_location_innoofwalls (Variables|Door|GetDoorY_Location_inNoOfWalls))
  (bind _window_rotationoffset (Variables|Window|GetWindow_RotationOffset))
  (bind _numofwallpiecerow (Variables|BuildingSize|GetNumOfWallPieceRow))
  (bind _numofwallpiecelength (Variables|BuildingSize|GetNumOfWallPieceLength))
  (bind (_outlocation _outrotator) (Utilities|SetOffsetforDirection _location_2 _doorlocationoffset _rotation_2 _door_rotationoffset PillarDirection))
  (bind (_outlocation_2 _outrotator_2) (Utilities|SetOffsetforDirection _location _windowlocationoffset _rotation _window_rotationoffset PillarDirection))
  (bind _returnvalue_3 (== Row_Index _doory_location_innoofwalls))
  (bind _returnvalue_4 (- _numofwallpiecerow 1))
  (bind _returnvalue_5 (- _numofwallpiecelength 1))
  (bind _returnvalue_6 (== Row_Index _doorx_location_innoofwalls))
  (bind _returnvalue_7 (and _returnvalue _returnvalue_3))
  (bind _returnvalue_8 (and _returnvalue_2 _returnvalue_6))
  (switch Utilities|FlowControl|Switch|SwitchonE_Type Type
    (:NewEnumerator0
      ;[1 1 1] Door
      (if (and (and (Utilities|Select :Index PillarDirection :NewEnumerator0 _returnvalue_8 :NewEnumerator1 _returnvalue_8 :NewEnumerator2 _returnvalue_7 :NewEnumerator3 _returnvalue_7) (Utilities|Select :Index PillarDirection :NewEnumerator0 (Variables|Door|GenerateDoor?|GetDoor_Front) :NewEnumerator1 (Variables|Door|GenerateDoor?|GetDoor_Back) :NewEnumerator2 (Variables|Door|GenerateDoor?|GetDoor_Left) :NewEnumerator3 (Variables|Door|GenerateDoor?|GetDoor_Right))) (!= Row_Index (Utilities|Select :Index PillarDirection :NewEnumerator0 _returnvalue_4 :NewEnumerator1 _returnvalue_4 :NewEnumerator2 _returnvalue_5 :NewEnumerator3 _returnvalue_5))) :!label _label
        (bind _meshcompref (Utilities|SpawnMesh (Math|Transform|MakeTransform _outlocation _outrotator (Variables|Door|GetDoorScale)) (Variables|StaticMesh|GetDoorMesh)))
        ;;[1 1 1] Set Remaining Offset
        (Variables|Default|SetRemainingLocationOffset _doorlocationoffset)
        (Variables|Window|SetLastPieceType "NewEnumerator2")
        (return _meshcompref)
        (else
          (bind _contains_ (Utilities|EvaluateLocationwithIndexes Height_Index Row_Index PillarDirection (Variables|Window|GetAlternativeWindowMode))
            (:Exe
              (if _contains_
                (bind _meshcompref_2 (Utilities|SpawnMesh (Math|Transform|MakeTransform _outlocation_2 _outrotator_2 (Variables|Window|GetWindowScale)) (Variables|StaticMesh|GetWindowMesh)))
                ;[1 1 1] Set Remaining Offset
                (Variables|Default|SetRemainingLocationOffset _windowlocationoffset)
                (Variables|Window|SetLastPieceType "NewEnumerator1")
                (return _meshcompref_2)
                (else
                  ;[1 1 1] wall
                  (Utilities|PositionOfMesh Height_Index
                    (:Lower
                      (bind _meshcompref_3 (Utilities|SpawnMesh (Math|Transform|MakeTransform (.OutLocation (Utilities|SetOffsetforDirection :BaseLocation _location_3 :LocationOffset (Utilities|Select :Index (Variables|Window|GetLastPieceType) :NewEnumerator0 (* (Variables|Default|GetRemainingLocationOffset) -1) :NewEnumerator1 "0, 0, 0" :NewEnumerator2 "0, 0, 0" :NewEnumerator4 "0, 0, 0" :NewEnumerator5 "0, 0, 0" :NewEnumerator6 "0, 0, 0" :NewEnumerator7 "0, 0, 0" :NewEnumerator8 "0, 0, 0") :Base%20Rotation _rotation_3 :Direction PillarDirection)) (.OutRotator (Utilities|SetOffsetforDirection :BaseLocation _location_3 :LocationOffset (Utilities|Select :Index (Variables|Window|GetLastPieceType) :NewEnumerator0 (* (Variables|Default|GetRemainingLocationOffset) -1) :NewEnumerator1 "0, 0, 0" :NewEnumerator2 "0, 0, 0" :NewEnumerator4 "0, 0, 0" :NewEnumerator5 "0, 0, 0" :NewEnumerator6 "0, 0, 0" :NewEnumerator7 "0, 0, 0" :NewEnumerator8 "0, 0, 0") :Base%20Rotation _rotation_3 :Direction PillarDirection)) _scale) (Variables|StaticMesh|Wall|GetLowerWallMesh)))
                      (Utilities|FlowControl|Sequence
                        (:then_0
                          _)
                        (:then_1
                          (return _meshcompref_3))))
                    (:Mid
                      (bind _meshcompref_4 (Utilities|SpawnMesh (Math|Transform|MakeTransform (.OutLocation (Utilities|SetOffsetforDirection :BaseLocation _location_3 :LocationOffset (Utilities|Select :Index (Variables|Window|GetLastPieceType) :NewEnumerator0 (* (Variables|Default|GetRemainingLocationOffset) -1) :NewEnumerator1 "0, 0, 0" :NewEnumerator2 "0, 0, 0" :NewEnumerator4 "0, 0, 0" :NewEnumerator5 "0, 0, 0" :NewEnumerator6 "0, 0, 0" :NewEnumerator7 "0, 0, 0" :NewEnumerator8 "0, 0, 0") :Base%20Rotation _rotation_3 :Direction PillarDirection)) (.OutRotator (Utilities|SetOffsetforDirection :BaseLocation _location_3 :LocationOffset (Utilities|Select :Index (Variables|Window|GetLastPieceType) :NewEnumerator0 (* (Variables|Default|GetRemainingLocationOffset) -1) :NewEnumerator1 "0, 0, 0" :NewEnumerator2 "0, 0, 0" :NewEnumerator4 "0, 0, 0" :NewEnumerator5 "0, 0, 0" :NewEnumerator6 "0, 0, 0" :NewEnumerator7 "0, 0, 0" :NewEnumerator8 "0, 0, 0") :Base%20Rotation _rotation_3 :Direction PillarDirection)) _scale) (Variables|StaticMesh|Wall|GetWallMesh)))
                      (Utilities|FlowControl|Sequence
                        (:then_0
                          _)
                        (:then_1
                          (return _meshcompref_4))))
                    (:Upper
                      (bind _meshcompref_5 (Utilities|SpawnMesh (Math|Transform|MakeTransform (.OutLocation (Utilities|SetOffsetforDirection :BaseLocation _location_3 :LocationOffset (Utilities|Select :Index (Variables|Window|GetLastPieceType) :NewEnumerator0 (* (Variables|Default|GetRemainingLocationOffset) -1) :NewEnumerator1 "0, 0, 0" :NewEnumerator2 "0, 0, 0" :NewEnumerator4 "0, 0, 0" :NewEnumerator5 "0, 0, 0" :NewEnumerator6 "0, 0, 0" :NewEnumerator7 "0, 0, 0" :NewEnumerator8 "0, 0, 0") :Base%20Rotation _rotation_3 :Direction PillarDirection)) (.OutRotator (Utilities|SetOffsetforDirection :BaseLocation _location_3 :LocationOffset (Utilities|Select :Index (Variables|Window|GetLastPieceType) :NewEnumerator0 (* (Variables|Default|GetRemainingLocationOffset) -1) :NewEnumerator1 "0, 0, 0" :NewEnumerator2 "0, 0, 0" :NewEnumerator4 "0, 0, 0" :NewEnumerator5 "0, 0, 0" :NewEnumerator6 "0, 0, 0" :NewEnumerator7 "0, 0, 0" :NewEnumerator8 "0, 0, 0") :Base%20Rotation _rotation_3 :Direction PillarDirection)) _scale) (Variables|StaticMesh|Wall|GetUpperWallMesh)))
                      (Utilities|FlowControl|Sequence
                        (:then_0
                          _)
                        (:then_1
                          (return _meshcompref_5)))))
                  ;[1 1 1] reset Remaining Offset
                  (Variables|Default|SetRemainingLocationOffset "0, 0, 0")
                  (Variables|Window|SetLastPieceType "NewEnumerator0"))))))))
    (:NewEnumerator1
      (goto _label))
    (:NewEnumerator2
      (goto _label))
    (:NewEnumerator4
      ;[1 1 1] Pillar
      (Utilities|PositionOfMesh Height_Index
        (:Lower
          (bind _meshcompref_6 (Utilities|SpawnMesh (Math|Transform|MakeTransform (.OutLocation (Utilities|SetOffsetforDirection (.Location (Math|Transform|BreakTransform (Math|Transform|MakeTransform (.OutLocation (Utilities|SetOffsetforDirection :BaseLocation _location_3 :LocationOffset (Utilities|Select :Index (Variables|Window|GetLastPieceType) :NewEnumerator0 (* (Variables|Default|GetRemainingLocationOffset) -1) :NewEnumerator1 "0, 0, 0" :NewEnumerator2 "0, 0, 0" :NewEnumerator4 "0, 0, 0" :NewEnumerator5 "0, 0, 0" :NewEnumerator6 "0, 0, 0" :NewEnumerator7 "0, 0, 0" :NewEnumerator8 "0, 0, 0") :Base%20Rotation _rotation_3 :Direction PillarDirection)) (.OutRotator (Utilities|SetOffsetforDirection :BaseLocation _location_3 :LocationOffset (Utilities|Select :Index (Variables|Window|GetLastPieceType) :NewEnumerator0 (* (Variables|Default|GetRemainingLocationOffset) -1) :NewEnumerator1 "0, 0, 0" :NewEnumerator2 "0, 0, 0" :NewEnumerator4 "0, 0, 0" :NewEnumerator5 "0, 0, 0" :NewEnumerator6 "0, 0, 0" :NewEnumerator7 "0, 0, 0" :NewEnumerator8 "0, 0, 0") :Base%20Rotation _rotation_3 :Direction PillarDirection)) _scale))) (Variables|Pillar|Lower|GetPillarLowerLocationOffset) (.Rotation (Math|Transform|BreakTransform (Math|Transform|MakeTransform (.OutLocation (Utilities|SetOffsetforDirection :BaseLocation _location_3 :LocationOffset (Utilities|Select :Index (Variables|Window|GetLastPieceType) :NewEnumerator0 (* (Variables|Default|GetRemainingLocationOffset) -1) :NewEnumerator1 "0, 0, 0" :NewEnumerator2 "0, 0, 0" :NewEnumerator4 "0, 0, 0" :NewEnumerator5 "0, 0, 0" :NewEnumerator6 "0, 0, 0" :NewEnumerator7 "0, 0, 0" :NewEnumerator8 "0, 0, 0") :Base%20Rotation _rotation_3 :Direction PillarDirection)) (.OutRotator (Utilities|SetOffsetforDirection :BaseLocation _location_3 :LocationOffset (Utilities|Select :Index (Variables|Window|GetLastPieceType) :NewEnumerator0 (* (Variables|Default|GetRemainingLocationOffset) -1) :NewEnumerator1 "0, 0, 0" :NewEnumerator2 "0, 0, 0" :NewEnumerator4 "0, 0, 0" :NewEnumerator5 "0, 0, 0" :NewEnumerator6 "0, 0, 0" :NewEnumerator7 "0, 0, 0" :NewEnumerator8 "0, 0, 0") :Base%20Rotation _rotation_3 :Direction PillarDirection)) _scale))) (Variables|Pillar|Lower|GetPillarLowerRotationOffset) PillarDirection)) (.OutRotator (Utilities|SetOffsetforDirection (.Location (Math|Transform|BreakTransform (Math|Transform|MakeTransform (.OutLocation (Utilities|SetOffsetforDirection :BaseLocation _location_3 :LocationOffset (Utilities|Select :Index (Variables|Window|GetLastPieceType) :NewEnumerator0 (* (Variables|Default|GetRemainingLocationOffset) -1) :NewEnumerator1 "0, 0, 0" :NewEnumerator2 "0, 0, 0" :NewEnumerator4 "0, 0, 0" :NewEnumerator5 "0, 0, 0" :NewEnumerator6 "0, 0, 0" :NewEnumerator7 "0, 0, 0" :NewEnumerator8 "0, 0, 0") :Base%20Rotation _rotation_3 :Direction PillarDirection)) (.OutRotator (Utilities|SetOffsetforDirection :BaseLocation _location_3 :LocationOffset (Utilities|Select :Index (Variables|Window|GetLastPieceType) :NewEnumerator0 (* (Variables|Default|GetRemainingLocationOffset) -1) :NewEnumerator1 "0, 0, 0" :NewEnumerator2 "0, 0, 0" :NewEnumerator4 "0, 0, 0" :NewEnumerator5 "0, 0, 0" :NewEnumerator6 "0, 0, 0" :NewEnumerator7 "0, 0, 0" :NewEnumerator8 "0, 0, 0") :Base%20Rotation _rotation_3 :Direction PillarDirection)) _scale))) (Variables|Pillar|Lower|GetPillarLowerLocationOffset) (.Rotation (Math|Transform|BreakTransform (Math|Transform|MakeTransform (.OutLocation (Utilities|SetOffsetforDirection :BaseLocation _location_3 :LocationOffset (Utilities|Select :Index (Variables|Window|GetLastPieceType) :NewEnumerator0 (* (Variables|Default|GetRemainingLocationOffset) -1) :NewEnumerator1 "0, 0, 0" :NewEnumerator2 "0, 0, 0" :NewEnumerator4 "0, 0, 0" :NewEnumerator5 "0, 0, 0" :NewEnumerator6 "0, 0, 0" :NewEnumerator7 "0, 0, 0" :NewEnumerator8 "0, 0, 0") :Base%20Rotation _rotation_3 :Direction PillarDirection)) (.OutRotator (Utilities|SetOffsetforDirection :BaseLocation _location_3 :LocationOffset (Utilities|Select :Index (Variables|Window|GetLastPieceType) :NewEnumerator0 (* (Variables|Default|GetRemainingLocationOffset) -1) :NewEnumerator1 "0, 0, 0" :NewEnumerator2 "0, 0, 0" :NewEnumerator4 "0, 0, 0" :NewEnumerator5 "0, 0, 0" :NewEnumerator6 "0, 0, 0" :NewEnumerator7 "0, 0, 0" :NewEnumerator8 "0, 0, 0") :Base%20Rotation _rotation_3 :Direction PillarDirection)) _scale))) (Variables|Pillar|Lower|GetPillarLowerRotationOffset) PillarDirection)) (Variables|Pillar|Lower|GetPillarScaleLower)) (Variables|StaticMesh|Pillar|GetLowerPillarMesh)))
          (Utilities|FlowControl|Sequence
            (:then_0
              _)
            (:then_1
              (return _meshcompref_6))))
        (:Mid
          (bind _meshcompref_7 (Utilities|SpawnMesh (Math|Transform|MakeTransform (.OutLocation (Utilities|SetOffsetforDirection (.Location (Math|Transform|BreakTransform (Math|Transform|MakeTransform (.OutLocation (Utilities|SetOffsetforDirection :BaseLocation _location_3 :LocationOffset (Utilities|Select :Index (Variables|Window|GetLastPieceType) :NewEnumerator0 (* (Variables|Default|GetRemainingLocationOffset) -1) :NewEnumerator1 "0, 0, 0" :NewEnumerator2 "0, 0, 0" :NewEnumerator4 "0, 0, 0" :NewEnumerator5 "0, 0, 0" :NewEnumerator6 "0, 0, 0" :NewEnumerator7 "0, 0, 0" :NewEnumerator8 "0, 0, 0") :Base%20Rotation _rotation_3 :Direction PillarDirection)) (.OutRotator (Utilities|SetOffsetforDirection :BaseLocation _location_3 :LocationOffset (Utilities|Select :Index (Variables|Window|GetLastPieceType) :NewEnumerator0 (* (Variables|Default|GetRemainingLocationOffset) -1) :NewEnumerator1 "0, 0, 0" :NewEnumerator2 "0, 0, 0" :NewEnumerator4 "0, 0, 0" :NewEnumerator5 "0, 0, 0" :NewEnumerator6 "0, 0, 0" :NewEnumerator7 "0, 0, 0" :NewEnumerator8 "0, 0, 0") :Base%20Rotation _rotation_3 :Direction PillarDirection)) _scale))) (Variables|Pillar|Mid|GetPillarLocationOffset) (.Rotation (Math|Transform|BreakTransform (Math|Transform|MakeTransform (.OutLocation (Utilities|SetOffsetforDirection :BaseLocation _location_3 :LocationOffset (Utilities|Select :Index (Variables|Window|GetLastPieceType) :NewEnumerator0 (* (Variables|Default|GetRemainingLocationOffset) -1) :NewEnumerator1 "0, 0, 0" :NewEnumerator2 "0, 0, 0" :NewEnumerator4 "0, 0, 0" :NewEnumerator5 "0, 0, 0" :NewEnumerator6 "0, 0, 0" :NewEnumerator7 "0, 0, 0" :NewEnumerator8 "0, 0, 0") :Base%20Rotation _rotation_3 :Direction PillarDirection)) (.OutRotator (Utilities|SetOffsetforDirection :BaseLocation _location_3 :LocationOffset (Utilities|Select :Index (Variables|Window|GetLastPieceType) :NewEnumerator0 (* (Variables|Default|GetRemainingLocationOffset) -1) :NewEnumerator1 "0, 0, 0" :NewEnumerator2 "0, 0, 0" :NewEnumerator4 "0, 0, 0" :NewEnumerator5 "0, 0, 0" :NewEnumerator6 "0, 0, 0" :NewEnumerator7 "0, 0, 0" :NewEnumerator8 "0, 0, 0") :Base%20Rotation _rotation_3 :Direction PillarDirection)) _scale))) (Variables|Pillar|Mid|GetPillarRotationOffset) PillarDirection)) (.OutRotator (Utilities|SetOffsetforDirection (.Location (Math|Transform|BreakTransform (Math|Transform|MakeTransform (.OutLocation (Utilities|SetOffsetforDirection :BaseLocation _location_3 :LocationOffset (Utilities|Select :Index (Variables|Window|GetLastPieceType) :NewEnumerator0 (* (Variables|Default|GetRemainingLocationOffset) -1) :NewEnumerator1 "0, 0, 0" :NewEnumerator2 "0, 0, 0" :NewEnumerator4 "0, 0, 0" :NewEnumerator5 "0, 0, 0" :NewEnumerator6 "0, 0, 0" :NewEnumerator7 "0, 0, 0" :NewEnumerator8 "0, 0, 0") :Base%20Rotation _rotation_3 :Direction PillarDirection)) (.OutRotator (Utilities|SetOffsetforDirection :BaseLocation _location_3 :LocationOffset (Utilities|Select :Index (Variables|Window|GetLastPieceType) :NewEnumerator0 (* (Variables|Default|GetRemainingLocationOffset) -1) :NewEnumerator1 "0, 0, 0" :NewEnumerator2 "0, 0, 0" :NewEnumerator4 "0, 0, 0" :NewEnumerator5 "0, 0, 0" :NewEnumerator6 "0, 0, 0" :NewEnumerator7 "0, 0, 0" :NewEnumerator8 "0, 0, 0") :Base%20Rotation _rotation_3 :Direction PillarDirection)) _scale))) (Variables|Pillar|Mid|GetPillarLocationOffset) (.Rotation (Math|Transform|BreakTransform (Math|Transform|MakeTransform (.OutLocation (Utilities|SetOffsetforDirection :BaseLocation _location_3 :LocationOffset (Utilities|Select :Index (Variables|Window|GetLastPieceType) :NewEnumerator0 (* (Variables|Default|GetRemainingLocationOffset) -1) :NewEnumerator1 "0, 0, 0" :NewEnumerator2 "0, 0, 0" :NewEnumerator4 "0, 0, 0" :NewEnumerator5 "0, 0, 0" :NewEnumerator6 "0, 0, 0" :NewEnumerator7 "0, 0, 0" :NewEnumerator8 "0, 0, 0") :Base%20Rotation _rotation_3 :Direction PillarDirection)) (.OutRotator (Utilities|SetOffsetforDirection :BaseLocation _location_3 :LocationOffset (Utilities|Select :Index (Variables|Window|GetLastPieceType) :NewEnumerator0 (* (Variables|Default|GetRemainingLocationOffset) -1) :NewEnumerator1 "0, 0, 0" :NewEnumerator2 "0, 0, 0" :NewEnumerator4 "0, 0, 0" :NewEnumerator5 "0, 0, 0" :NewEnumerator6 "0, 0, 0" :NewEnumerator7 "0, 0, 0" :NewEnumerator8 "0, 0, 0") :Base%20Rotation _rotation_3 :Direction PillarDirection)) _scale))) (Variables|Pillar|Mid|GetPillarRotationOffset) PillarDirection)) (Variables|Pillar|Mid|GetPillarScale)) (Variables|StaticMesh|Pillar|GetPillarMesh)))
          (Utilities|FlowControl|Sequence
            (:then_0
              _)
            (:then_1
              (return _meshcompref_7))))
        (:Upper
          (bind _meshcompref_8 (Utilities|SpawnMesh (Math|Transform|MakeTransform (.OutLocation (Utilities|SetOffsetforDirection (.Location (Math|Transform|BreakTransform (Math|Transform|MakeTransform (.OutLocation (Utilities|SetOffsetforDirection :BaseLocation _location_3 :LocationOffset (Utilities|Select :Index (Variables|Window|GetLastPieceType) :NewEnumerator0 (* (Variables|Default|GetRemainingLocationOffset) -1) :NewEnumerator1 "0, 0, 0" :NewEnumerator2 "0, 0, 0" :NewEnumerator4 "0, 0, 0" :NewEnumerator5 "0, 0, 0" :NewEnumerator6 "0, 0, 0" :NewEnumerator7 "0, 0, 0" :NewEnumerator8 "0, 0, 0") :Base%20Rotation _rotation_3 :Direction PillarDirection)) (.OutRotator (Utilities|SetOffsetforDirection :BaseLocation _location_3 :LocationOffset (Utilities|Select :Index (Variables|Window|GetLastPieceType) :NewEnumerator0 (* (Variables|Default|GetRemainingLocationOffset) -1) :NewEnumerator1 "0, 0, 0" :NewEnumerator2 "0, 0, 0" :NewEnumerator4 "0, 0, 0" :NewEnumerator5 "0, 0, 0" :NewEnumerator6 "0, 0, 0" :NewEnumerator7 "0, 0, 0" :NewEnumerator8 "0, 0, 0") :Base%20Rotation _rotation_3 :Direction PillarDirection)) _scale))) (Variables|Pillar|Upper|GetPillarUpperLocationOffset) (.Rotation (Math|Transform|BreakTransform (Math|Transform|MakeTransform (.OutLocation (Utilities|SetOffsetforDirection :BaseLocation _location_3 :LocationOffset (Utilities|Select :Index (Variables|Window|GetLastPieceType) :NewEnumerator0 (* (Variables|Default|GetRemainingLocationOffset) -1) :NewEnumerator1 "0, 0, 0" :NewEnumerator2 "0, 0, 0" :NewEnumerator4 "0, 0, 0" :NewEnumerator5 "0, 0, 0" :NewEnumerator6 "0, 0, 0" :NewEnumerator7 "0, 0, 0" :NewEnumerator8 "0, 0, 0") :Base%20Rotation _rotation_3 :Direction PillarDirection)) (.OutRotator (Utilities|SetOffsetforDirection :BaseLocation _location_3 :LocationOffset (Utilities|Select :Index (Variables|Window|GetLastPieceType) :NewEnumerator0 (* (Variables|Default|GetRemainingLocationOffset) -1) :NewEnumerator1 "0, 0, 0" :NewEnumerator2 "0, 0, 0" :NewEnumerator4 "0, 0, 0" :NewEnumerator5 "0, 0, 0" :NewEnumerator6 "0, 0, 0" :NewEnumerator7 "0, 0, 0" :NewEnumerator8 "0, 0, 0") :Base%20Rotation _rotation_3 :Direction PillarDirection)) _scale))) (Variables|Pillar|Upper|GetPillarUpperRotationOffset) PillarDirection)) (.OutRotator (Utilities|SetOffsetforDirection (.Location (Math|Transform|BreakTransform (Math|Transform|MakeTransform (.OutLocation (Utilities|SetOffsetforDirection :BaseLocation _location_3 :LocationOffset (Utilities|Select :Index (Variables|Window|GetLastPieceType) :NewEnumerator0 (* (Variables|Default|GetRemainingLocationOffset) -1) :NewEnumerator1 "0, 0, 0" :NewEnumerator2 "0, 0, 0" :NewEnumerator4 "0, 0, 0" :NewEnumerator5 "0, 0, 0" :NewEnumerator6 "0, 0, 0" :NewEnumerator7 "0, 0, 0" :NewEnumerator8 "0, 0, 0") :Base%20Rotation _rotation_3 :Direction PillarDirection)) (.OutRotator (Utilities|SetOffsetforDirection :BaseLocation _location_3 :LocationOffset (Utilities|Select :Index (Variables|Window|GetLastPieceType) :NewEnumerator0 (* (Variables|Default|GetRemainingLocationOffset) -1) :NewEnumerator1 "0, 0, 0" :NewEnumerator2 "0, 0, 0" :NewEnumerator4 "0, 0, 0" :NewEnumerator5 "0, 0, 0" :NewEnumerator6 "0, 0, 0" :NewEnumerator7 "0, 0, 0" :NewEnumerator8 "0, 0, 0") :Base%20Rotation _rotation_3 :Direction PillarDirection)) _scale))) (Variables|Pillar|Upper|GetPillarUpperLocationOffset) (.Rotation (Math|Transform|BreakTransform (Math|Transform|MakeTransform (.OutLocation (Utilities|SetOffsetforDirection :BaseLocation _location_3 :LocationOffset (Utilities|Select :Index (Variables|Window|GetLastPieceType) :NewEnumerator0 (* (Variables|Default|GetRemainingLocationOffset) -1) :NewEnumerator1 "0, 0, 0" :NewEnumerator2 "0, 0, 0" :NewEnumerator4 "0, 0, 0" :NewEnumerator5 "0, 0, 0" :NewEnumerator6 "0, 0, 0" :NewEnumerator7 "0, 0, 0" :NewEnumerator8 "0, 0, 0") :Base%20Rotation _rotation_3 :Direction PillarDirection)) (.OutRotator (Utilities|SetOffsetforDirection :BaseLocation _location_3 :LocationOffset (Utilities|Select :Index (Variables|Window|GetLastPieceType) :NewEnumerator0 (* (Variables|Default|GetRemainingLocationOffset) -1) :NewEnumerator1 "0, 0, 0" :NewEnumerator2 "0, 0, 0" :NewEnumerator4 "0, 0, 0" :NewEnumerator5 "0, 0, 0" :NewEnumerator6 "0, 0, 0" :NewEnumerator7 "0, 0, 0" :NewEnumerator8 "0, 0, 0") :Base%20Rotation _rotation_3 :Direction PillarDirection)) _scale))) (Variables|Pillar|Upper|GetPillarUpperRotationOffset) PillarDirection)) (Variables|Pillar|Upper|GetPillarScaleUpper)) (Variables|StaticMesh|Pillar|GetUpperPillarMesh)))
          (Utilities|FlowControl|Sequence
            (:then_0
              _)
            (:then_1
              (return _meshcompref_8)))))
      ;[1 1 1] reset Remaining Offset
      (Variables|Default|SetRemainingLocationOffset "0, 0, 0")
      (Variables|Default|SetRemainingRotationOffset "0, 0, 0")
      (Variables|Window|SetLastPieceType "NewEnumerator4"))))

(fn BakeMesh
  (bind _returnvalue (Game|SpawnActorfromClass "/Script/Engine.LightWeightInstanceStaticMeshManager" (Transformation|GetActorTransform) "Undefined" 0 0))
  (for _array_element (Components|GetChildrenComponents (Variables|Default|GetDefaultSceneRoot) false)
    (bind _asstatic_mesh_component (Utilities|Casting|CastToStaticMeshComponent _array_element))
    (Utilities|IsValid _asstatic_mesh_component
      (:Is%20Valid
        (Components|InstancedStaticMesh|AddInstance (Variables|/Script/Engine.LightWeightInstanceStaticMeshManager|GetInstancedStaticMeshComponent _returnvalue) (Transformation|GetWorldTransform _array_element) true)
        (Components|StaticMesh|SetStaticMesh (Variables|/Script/Engine.LightWeightInstanceStaticMeshManager|GetInstancedStaticMeshComponent _returnvalue) (Variables|/Script/Engine.StaticMeshComponent|GetStaticMesh _asstatic_mesh_component))))))
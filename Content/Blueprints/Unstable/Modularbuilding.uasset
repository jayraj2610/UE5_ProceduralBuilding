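; Procedural modular building actor that assembles a rectangular shell from static mesh tiles in its Construction Script, sized by row, length and height counts.
; It builds front, right, back and left walls in turn, placing each floor's tiles from the previous side's corner and alternating two corner arrays.
; A helper picks lower, middle or upper meshes by floor, offsets corners, and adds each piece as a StaticMeshComponent.
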(event EventBeginPlay)

(fn ConstructionScript
  (Utilities|FlowControl|Sequence
    (:then_0
      (Variables|Default|SetStartLocation (Transformation|GetRelativeTransform (Variables|Default|GetDefaultSceneRoot))))
    (:then_1
      ;[1 1 1] Front
      (for _index (range 1 (Variables|BuildingSize|GetNumOfMiddlePieceHeight))
        (bind _meshcompref (CallFunction|HandleTypeandSpawnMeshComp (Math|Transform|MakeTransform (+ (.location (Variables|Default|GetStartLocation)) (Math|Vector|MakeVector 0.0 0.0 (* _index (Variables|AssetSize|GetCornerZ_Height)))) (.rotation (Variables|Default|GetStartLocation)) "1.000000,1.000000,1.000000") true _index false))
        (bind _returnvalue (Utilities|Array|Add (Variables|Default|GetCornerStartArrayRef) _meshcompref))
        (Variables|Default|SetCurrentCornerNum _returnvalue)
        (for _index_2 (range 1 (Variables|BuildingSize|GetNumOfMiddlePieceRow))
          (bind _meshcompref_2 (CallFunction|HandleTypeandSpawnMeshComp (Math|Transform|MakeTransform (+ (Math|Vector|MakeVector (* (Variables|AssetSize|GetMiddlePieceXWidth) (- _index_2 1)) 0.0 0.0) (Math|Vector|MakeVector (Variables|AssetSize|GetCornerX_Width) 0.0 0.0) (.Location (Utilities|RemoveCornerOffset (Transformation|GetRelativeTransform (Utilities|Array|Get(acopy) (Variables|Default|GetCornerStartArrayRef) (Variables|Default|GetCurrentCornerNum)))))) (.Rotation (Utilities|RemoveCornerOffset (Transformation|GetRelativeTransform (Utilities|Array|Get(acopy) (Variables|Default|GetCornerStartArrayRef) (Variables|Default|GetCurrentCornerNum))))) "1.000000,1.000000,1.000000") false _index false))
          (Variables|Default|SetLastTile _meshcompref_2))
        ;;[1 1 1] LoopEndCroner
        (bind _meshcompref_3 (CallFunction|HandleTypeandSpawnMeshComp (Math|Transform|MakeTransform (+ (Utilities|FixLocationOffset (.location (Transformation|GetRelativeTransform (Variables|Default|GetLastTile))) "NewEnumerator0") (Math|Vector|MakeVector (* (Variables|AssetSize|GetMiddlePieceXWidth) 2.0) 0.0 0.0) "") (Math|Rotator|CombineRotators (.rotation (Transformation|GetRelativeTransform (Variables|Default|GetLastTile))) "0.000000,-90.000000,0.000000") "1.000000,1.000000,1.000000") true _index false))
        (Utilities|Array|Add (Variables|Default|GetCornerEndArrayRef) _meshcompref_3))
      (Utilities|Array|Clear (Variables|Default|GetCornerStartArrayRef))
      ;[1 1 1] right
      (for _index_3 (range 1 (Variables|BuildingSize|GetNumOfMiddlePieceHeight))
        (Variables|Default|SetCurrentCornerNum (- _index_3 1))
        (for _index_4 (range 1 (Variables|BuildingSize|GetNumOfMiddlePieceLength))
          (bind _meshcompref_4 (CallFunction|HandleTypeandSpawnMeshComp (Math|Transform|MakeTransform (+ (Math|Vector|MakeVector 0.0 (* (* (Variables|AssetSize|GetMiddlePieceXWidth) (- _index_4 1)) -1.0) 0.0) (Math|Vector|MakeVector 0.0 (* (Variables|AssetSize|GetCornerX_Width) -1.0) 0.0) (.Location (Utilities|RemoveCornerOffset (Math|Transform|MakeTransform (.location (Transformation|GetRelativeTransform (Utilities|Array|Get(acopy) (Variables|Default|GetCornerEndArrayRef) (Variables|Default|GetCurrentCornerNum)))) (.rotation (Transformation|GetRelativeTransform (Utilities|Array|Get(acopy) (Variables|Default|GetCornerEndArrayRef) (Variables|Default|GetCurrentCornerNum)))) (.scale (Transformation|GetRelativeTransform (Utilities|Array|Get(acopy) (Variables|Default|GetCornerEndArrayRef) (Variables|Default|GetCurrentCornerNum)))))))) (.Rotation (Utilities|RemoveCornerOffset (Math|Transform|MakeTransform (.location (Transformation|GetRelativeTransform (Utilities|Array|Get(acopy) (Variables|Default|GetCornerEndArrayRef) (Variables|Default|GetCurrentCornerNum)))) (.rotation (Transformation|GetRelativeTransform (Utilities|Array|Get(acopy) (Variables|Default|GetCornerEndArrayRef) (Variables|Default|GetCurrentCornerNum)))) (.scale (Transformation|GetRelativeTransform (Utilities|Array|Get(acopy) (Variables|Default|GetCornerEndArrayRef) (Variables|Default|GetCurrentCornerNum))))))) "1.000000,1.000000,1.000000") false _index_3 false))
          (Variables|Default|SetLastTile _meshcompref_4))
        ;;[1 1 1] LoopEndCroner
        (bind _meshcompref_5 (CallFunction|HandleTypeandSpawnMeshComp (Math|Transform|MakeTransform (+ (.location (Transformation|GetRelativeTransform (Variables|Default|GetLastTile))) (Math|Vector|MakeVector 0.0 (* (Variables|AssetSize|GetMiddlePieceXWidth) -2.0) 0.0)) (Math|Rotator|CombineRotators (.rotation (Transformation|GetRelativeTransform (Variables|Default|GetLastTile))) "0.000000,-90.000000,0.000000") "1.000000,1.000000,1.000000") true _index_3 false))
        (Utilities|Array|Add (Variables|Default|GetCornerStartArrayRef) _meshcompref_5))
      (Utilities|Array|Clear (Variables|Default|GetCornerEndArrayRef))
      ;[1 1 1] back
      (for _index_5 (range 1 (Variables|BuildingSize|GetNumOfMiddlePieceHeight))
        (Variables|Default|SetCurrentCornerNum (- _index_5 1))
        (for _index_6 (range 1 (Variables|BuildingSize|GetNumOfMiddlePieceRow))
          (bind _meshcompref_6 (CallFunction|HandleTypeandSpawnMeshComp (Math|Transform|MakeTransform (+ (Math|Vector|MakeVector (* (* (Variables|AssetSize|GetMiddlePieceXWidth) (- _index_6 1)) -1.0) 0.0 0.0) (Math|Vector|MakeVector (* (Variables|AssetSize|GetCornerX_Width) -1.0) 0.0 0.0) (.Location (Utilities|RemoveCornerOffset (Transformation|GetRelativeTransform (Utilities|Array|Get(acopy) (Variables|Default|GetCornerStartArrayRef) (Variables|Default|GetCurrentCornerNum)))))) (.Rotation (Utilities|RemoveCornerOffset (Transformation|GetRelativeTransform (Utilities|Array|Get(acopy) (Variables|Default|GetCornerStartArrayRef) (Variables|Default|GetCurrentCornerNum))))) "1.000000,1.000000,1.000000") false _index_5 false))
          (Variables|Default|SetLastTile _meshcompref_6))
        ;;[1 1 1] LoopEndCroner
        (bind _meshcompref_7 (CallFunction|HandleTypeandSpawnMeshComp (Math|Transform|MakeTransform (+ (.location (Transformation|GetRelativeTransform (Variables|Default|GetLastTile))) (Math|Vector|MakeVector (* (Variables|AssetSize|GetMiddlePieceXWidth) -2.0) 0.0 0.0)) (Math|Rotator|CombineRotators (.rotation (Transformation|GetRelativeTransform (Variables|Default|GetLastTile))) "0.000000,-90.000000,0.000000") "1.000000,1.000000,1.000000") true _index_5 false))
        (Utilities|Array|Add (Variables|Default|GetCornerEndArrayRef) _meshcompref_7))
      (Utilities|Array|Clear (Variables|Default|GetCornerStartArrayRef))
      ;[1 1 1] Left
      (for _index_7 (range 1 (Variables|BuildingSize|GetNumOfMiddlePieceHeight))
        (Variables|Default|SetCurrentCornerNum (- _index_7 1))
        (for _index_8 (range 1 (Variables|BuildingSize|GetNumOfMiddlePieceLength))
          (bind _meshcompref_8 (CallFunction|HandleTypeandSpawnMeshComp (Math|Transform|MakeTransform (+ (Math|Vector|MakeVector 0.0 (* (Variables|AssetSize|GetMiddlePieceXWidth) (- _index_8 1)) 0.0) (Math|Vector|MakeVector 0.0 (Variables|AssetSize|GetCornerX_Width) 0.0) (.Location (Utilities|RemoveCornerOffset (Transformation|GetRelativeTransform (Utilities|Array|Get(acopy) (Variables|Default|GetCornerEndArrayRef) (Variables|Default|GetCurrentCornerNum)))))) (.Rotation (Utilities|RemoveCornerOffset (Transformation|GetRelativeTransform (Utilities|Array|Get(acopy) (Variables|Default|GetCornerEndArrayRef) (Variables|Default|GetCurrentCornerNum))))) "1.000000,1.000000,1.000000") false _index_7 false))
          (Variables|Default|SetLastTile _meshcompref_8))))))

(fn HandleTypeandSpawnMeshComp
  (params (Transform :type Transform) (isCorner :type Boolean) (CounterIndex :type Integer) (First%20timeGenratingCorner :type Boolean))
  (bind (_location _rotation _scale) (Math|Transform|BreakTransform Transform))
  (bind _cornerrotationoffset (Variables|Offset|GetCornerRotationOffset))
  (bind _cornerlocationoffset (Variables|Offset|GetCornerLocationOffset))
  (bind _returnvalue (Math|Rotator|CombineRotators _rotation _cornerrotationoffset))
  (bind _returnvalue_2 (+ _location _cornerlocationoffset))
  (bind _returnvalue_3 (Math|Transform|MakeTransform _returnvalue_2 _returnvalue _scale))
  (if isCorner
    (Utilities|Position CounterIndex
      (:Lower
        (bind _meshcompref (Utilities|SpawnMesh _returnvalue_3 (Variables|StaticMesh|GetLowerCornerMesh)))
        (return _meshcompref))
      (:Mid
        (bind _meshcompref_2 (Utilities|SpawnMesh _returnvalue_3 (Variables|StaticMesh|GetCornerMesh)))
        (return _meshcompref_2))
      (:Upper
        (bind _meshcompref_3 (Utilities|SpawnMesh _returnvalue_3 (Variables|StaticMesh|GetUpperCornerMesh)))
        (return _meshcompref_3)))
    (else
      (Utilities|Position CounterIndex
        (:Lower
          (bind _meshcompref_4 (Utilities|SpawnMesh Transform (Variables|StaticMesh|GetLowerMidTileMesh)))
          (return _meshcompref_4))
        (:Mid
          (bind _meshcompref_5 (Utilities|SpawnMesh Transform (Variables|StaticMesh|GetMidTileMesh)))
          (return _meshcompref_5))
        (:Upper
          (bind _meshcompref_6 (Utilities|SpawnMesh Transform (Variables|StaticMesh|GetUpperMidTileMesh)))
          (return _meshcompref_6))))))
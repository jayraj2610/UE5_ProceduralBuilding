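; Procedural modular building actor that assembles a rectangular shell from static mesh components in the Construction Script, sized by row, length and height piece counts.
; Four wall loops chain around the perimeter from each side's last tile, choosing lower, middle or upper meshes by floor index.
; Those end tiles also anchor optional corner pillars with direction-adjusted offsets.
; Optional grids fill roof and floor, and each row's end walls can be destroyed or hidden.
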(event EventBeginPlay)

(fn ConstructionScript
  (bind _wallx_width (Variables|AssetSize|GetWallX_Width))
  (bind _defaultsceneroot (Variables|Default|GetDefaultSceneRoot))
  (bind _wallx_width_2 (Variables|AssetSize|GetWallX_Width))
  (bind _wallx_width_3 (Variables|AssetSize|GetWallX_Width))
  (bind _returnvalue (Transformation|GetRelativeTransform _defaultsceneroot))
  (Utilities|FlowControl|Sequence
    (:then_0
      (Variables|Default|SetStartLocation (Math|Transform|MakeTransform (Transformation|GetWorldLocation (Variables|Default|GetDefaultSceneRoot)) (.rotation _returnvalue) (.scale _returnvalue))))
    (:then_1
      ;[1 1 1] Front X+
      (for _index (range 0 (- (Variables|BuildingSize|GetNumOfMiddlePieceHeight) 1))
        (for _index_2 (range 0 (- (Variables|BuildingSize|GetNumOfMiddlePieceRow) 1))
          (bind _meshcompref (CallFunction|HandleTypeandSpawnMeshComp (Math|Transform|MakeTransform (+ (Math|Vector|MakeVector (* _index_2 (Variables|AssetSize|GetWallX_Width)) 0.0 (* _index (Variables|AssetSize|GetWallZ_Height))) (.location (Variables|Default|GetStartLocation))) (.rotation (Variables|Default|GetStartLocation)) "1.000000,1.000000,1.000000") _index false "NewEnumerator0"))
          (bind _output_get (Variables|Default|SetLastTile _meshcompref))
          (Utilities|SaveFirstandLastWallOfRow _output_get _index_2 true))
        (Utilities|Array|Add (Variables|Default|GetLastTileArray) (Variables|Default|GetLastTile))
        (Utilities|Array|Add (Variables|Pillar|GetPillar_1_Transform) (Transformation|GetRelativeTransform (Variables|Default|GetLastTile))))
      ;[1 1 1] Right Y-
      (for _index_3 (range 0 (- (Variables|BuildingSize|GetNumOfMiddlePieceHeight) 1))
        (for _index_4 (range 0 (- (Variables|BuildingSize|GetNumOfMiddlePieceLength) 1))
          (bind _meshcompref_2 (CallFunction|HandleTypeandSpawnMeshComp (Math|Transform|MakeTransform (select (== _index_4 0) (+ (Math|Vector|MakeVector _wallx_width_3 0.0 0.0) (.location (Transformation|GetRelativeTransform (Utilities|Array|Get(acopy) (Variables|Default|GetLastTileArray) _index_3)))) (+ (.location (Transformation|GetRelativeTransform (Variables|Default|GetLastTile))) (Math|Vector|MakeVector 0.0 (* _wallx_width_3 -1.0) 0.0))) (Math|Rotator|CombineRotators (.rotation (Transformation|GetRelativeTransform (Utilities|Array|Get(acopy) (Variables|Default|GetLastTileArray) _index_3))) "0.000000,-90.000000,0.000000") "1.000000,1.000000,1.000000") _index_3 false "NewEnumerator0"))
          (bind _output_get_2 (Variables|Default|SetLastTile _meshcompref_2))
          (Utilities|SaveFirstandLastWallOfRow _output_get_2 _index_4 false))
        (Utilities|Array|Add (Variables|Default|GetLastTileArray2) (Variables|Default|GetLastTile))
        (Utilities|Array|Add (Variables|Pillar|GetPillar_2_Transform) (Transformation|GetRelativeTransform (Variables|Default|GetLastTile))))
      (Utilities|Array|Clear (Variables|Default|GetLastTileArray))
      ;[1 1 1] Back X-
      (for _index_5 (range 0 (- (Variables|BuildingSize|GetNumOfMiddlePieceHeight) 1))
        (for _index_6 (range 0 (- (Variables|BuildingSize|GetNumOfMiddlePieceRow) 1))
          (bind _meshcompref_3 (CallFunction|HandleTypeandSpawnMeshComp (Math|Transform|MakeTransform (select (== _index_6 0) (+ (Math|Vector|MakeVector 0.0 (* _wallx_width -1.0) 0.0) (.location (Transformation|GetRelativeTransform (Utilities|Array|Get(acopy) (Variables|Default|GetLastTileArray2) _index_5)))) (+ (.location (Transformation|GetRelativeTransform (Variables|Default|GetLastTile))) (Math|Vector|MakeVector (* _wallx_width -1.0) 0.0 0.0))) (Math|Rotator|CombineRotators (.rotation (Transformation|GetRelativeTransform (Utilities|Array|Get(acopy) (Variables|Default|GetLastTileArray2) _index_5))) "0.000000,-90.000000,0.000000") "1.000000,1.000000,1.000000") _index_5 false "NewEnumerator0"))
          (bind _output_get_3 (Variables|Default|SetLastTile _meshcompref_3))
          (Utilities|SaveFirstandLastWallOfRow _output_get_3 _index_6 true))
        (Utilities|Array|Add (Variables|Default|GetLastTileArray) (Variables|Default|GetLastTile))
        (Utilities|Array|Add (Variables|Pillar|GetPillar_3_Transform) (Transformation|GetRelativeTransform (Variables|Default|GetLastTile))))
      (Utilities|Array|Clear (Variables|Default|GetLastTileArray2))
      ;[1 1 1] Left Y+
      (for _index_7 (range 0 (- (Variables|BuildingSize|GetNumOfMiddlePieceHeight) 1))
        (for _index_8 (range 0 (- (Variables|BuildingSize|GetNumOfMiddlePieceLength) 1))
          (bind _meshcompref_4 (CallFunction|HandleTypeandSpawnMeshComp (Math|Transform|MakeTransform (select (== _index_8 0) (+ (Math|Vector|MakeVector (* _wallx_width_2 -1.0) 0.0 0.0) (.location (Transformation|GetRelativeTransform (Utilities|Array|Get(acopy) (Variables|Default|GetLastTileArray) _index_7)))) (+ (.location (Transformation|GetRelativeTransform (Variables|Default|GetLastTile))) (Math|Vector|MakeVector 0.0 _wallx_width_2 0.0))) (Math|Rotator|CombineRotators (.rotation (Transformation|GetRelativeTransform (Utilities|Array|Get(acopy) (Variables|Default|GetLastTileArray) _index_7))) "0.000000,-90.000000,0.000000") "1.000000,1.000000,1.000000") _index_7 false "NewEnumerator0"))
          (bind _output_get_4 (Variables|Default|SetLastTile _meshcompref_4))
          (Utilities|SaveFirstandLastWallOfRow _output_get_4 _index_8 false))
        (Utilities|Array|Add (Variables|Default|GetLastTileArray2) (Variables|Default|GetLastTile))
        (Utilities|Array|Add (Variables|Pillar|GetPillar_4_Transform) (Transformation|GetRelativeTransform (Variables|Default|GetLastTile))))
      (Utilities|Array|Clear (Variables|Default|GetLastTileArray))
      (Utilities|FlowControl|Sequence
        (:then_0
          (Utilities|FlowControl|Sequence
            (:then_0
              (if (Variables|Roof|GetGenerate%20Roof)
                ;[1 1 1] Roof
                (for _index_9 (range 0 (- (Variables|BuildingSize|GetNumOfMiddlePieceLength) 1))
                  (for _index_10 (range 0 (- (Variables|BuildingSize|GetNumOfMiddlePieceRow) 1))
                    (Utilities|SpawnMesh (Math|Transform|MakeTransform (+ (.location (Variables|Default|GetStartLocation)) (Math|Vector|MakeVector (* _index_10 (Variables|AssetSize|GetWallX_Width)) (* _index_9 (Variables|AssetSize|GetWallZ_Height) -1.0) (+ (* (Variables|AssetSize|GetWallZ_Height) (Variables|BuildingSize|GetNumOfMiddlePieceHeight)) (Variables|Roof|GetRoofZOffset)))) (Math|Rotator|CombineRotators (Math|Rotator|CombineRotators (.rotation (Variables|Default|GetStartLocation)) "0.000000,0.000000,180.000000") (Variables|Roof|GetRoofRotationOffset)) (Variables|Roof|GetRoofScale)) (Variables|StaticMesh|GetRoofMesh))))))
            (:then_1
              (if (Variables|Floor|GetGenerate%20Floor)
                ;[1 1 1] Floor
                (for _index_11 (range 0 (- (Variables|BuildingSize|GetNumOfMiddlePieceLength) 1))
                  (for _index_12 (range 0 (- (Variables|BuildingSize|GetNumOfMiddlePieceRow) 1))
                    (Utilities|SpawnMesh (Math|Transform|MakeTransform (+ (.location (Variables|Default|GetStartLocation)) (Math|Vector|MakeVector (* _index_12 (Variables|AssetSize|GetWallX_Width)) (* _index_11 (Variables|AssetSize|GetWallZ_Height) -1.0) (Variables|Floor|GetFloorZOffset))) (Math|Rotator|CombineRotators (Math|Rotator|CombineRotators (.rotation (Variables|Default|GetStartLocation)) "0.000000,0.000000,180.000000") (Variables|Floor|GetFloorRotationOffset)) (Variables|Floor|GetFloorScale)) (Variables|StaticMesh|GetFloorMesh))))))))
        (:then_1
          (if (Variables|Pillar|GetGenerate%20Pillar)
            (Utilities|FlowControl|Sequence
              (:then_0
                ;[1 1 1] Pillar1 Front
                (for _index_13 (range 0 (- (Variables|BuildingSize|GetNumOfMiddlePieceHeight) 1))
                  (CallFunction|HandleTypeandSpawnMeshComp (Math|Transform|MakeTransform (+ (.location (Utilities|Array|Get(acopy) (Variables|Pillar|GetPillar_1_Transform) _index_13)) (Math|Vector|MakeVector 0.0 0.0 0.0)) (.rotation (Utilities|Array|Get(acopy) (Variables|Pillar|GetPillar_1_Transform) _index_13)) (Variables|Pillar|Mid|GetPillarScale)) _index_13 true "NewEnumerator0")))
              (:then_1
                ;[1 1 1] Pillar2 Right
                (for _index_14 (range 0 (- (Variables|BuildingSize|GetNumOfMiddlePieceHeight) 1))
                  (CallFunction|HandleTypeandSpawnMeshComp (Math|Transform|MakeTransform (+ (.location (Utilities|Array|Get(acopy) (Variables|Pillar|GetPillar_2_Transform) _index_14)) (Math|Vector|MakeVector 0.0 0.0 0.0)) (.rotation (Utilities|Array|Get(acopy) (Variables|Pillar|GetPillar_2_Transform) _index_14)) (Variables|Pillar|Mid|GetPillarScale)) _index_14 true "NewEnumerator3")))
              (:then_2
                ;[1 1 1] Pillar3 Back
                (for _index_15 (range 0 (- (Variables|BuildingSize|GetNumOfMiddlePieceHeight) 1))
                  (CallFunction|HandleTypeandSpawnMeshComp (Math|Transform|MakeTransform (+ (.location (Utilities|Array|Get(acopy) (Variables|Pillar|GetPillar_3_Transform) _index_15)) (Math|Vector|MakeVector 0.0 0.0 0.0)) (.rotation (Utilities|Array|Get(acopy) (Variables|Pillar|GetPillar_3_Transform) _index_15)) (Variables|Pillar|Mid|GetPillarScale)) _index_15 true "NewEnumerator1")))
              (:then_3
                ;[1 1 1] Pillar4 Left
                (for _index_16 (range 0 (- (Variables|BuildingSize|GetNumOfMiddlePieceHeight) 1))
                  (CallFunction|HandleTypeandSpawnMeshComp (Math|Transform|MakeTransform (+ (.location (Utilities|Array|Get(acopy) (Variables|Pillar|GetPillar_4_Transform) _index_16)) (Math|Vector|MakeVector 0.0 0.0 0.0)) (.rotation (Utilities|Array|Get(acopy) (Variables|Pillar|GetPillar_4_Transform) _index_16)) (Variables|Pillar|Mid|GetPillarScale)) _index_16 true "NewEnumerator2"))))))
        (:then_2
          (Utilities|HandleFirstandLastWallOFRows))))))

(fn HandleTypeandSpawnMeshComp
  (params (Transform :type Transform) (CounterIndex :type Integer) (Is%20Pillar :type Boolean) (PillarDirection :type E_Direction%20Enum :default "NewEnumerator0"))
  (bind (_location _rotation) (Math|Transform|BreakTransform Transform))
  (bind (_location_2 _rotation_2) (Math|Transform|BreakTransform Transform))
  (bind (_location_3 _rotation_3) (Math|Transform|BreakTransform Transform))
  (bind _pillarlowerlocationoffset (Variables|Pillar|Lower|GetPillarLowerLocationOffset))
  (bind _pillarlocationoffset (Variables|Pillar|Mid|GetPillarLocationOffset))
  (bind _pillarupperlocationoffset (Variables|Pillar|Upper|GetPillarUpperLocationOffset))
  (bind _pillarlowerrotationoffset (Variables|Pillar|Lower|GetPillarLowerRotationOffset))
  (bind _pillarrotationoffset (Variables|Pillar|Mid|GetPillarRotationOffset))
  (bind _pillarupperrotationoffset (Variables|Pillar|Upper|GetPillarUpperRotationOffset))
  (bind (_outlocation _outrotator) (Utilities|SetOffsetforDirection _location_2 _pillarlocationoffset _rotation_2 _pillarrotationoffset PillarDirection))
  (bind (_outlocation_2 _outrotator_2) (Utilities|SetOffsetforDirection _location _pillarupperlocationoffset _rotation _pillarupperrotationoffset PillarDirection))
  (bind (_outlocation_3 _outrotator_3) (Utilities|SetOffsetforDirection _location_3 _pillarlowerlocationoffset _rotation_3 _pillarlowerrotationoffset PillarDirection))
  (if Is%20Pillar
    (Utilities|PositionOfMesh CounterIndex
      (:Lower
        (bind _meshcompref (Utilities|SpawnMesh (Math|Transform|MakeTransform _outlocation_3 _outrotator_3 (Variables|Pillar|Lower|GetPillarScaleLower)) (Variables|StaticMesh|GetLowerPillarMesh)))
        (return _meshcompref))
      (:Mid
        (bind _meshcompref_2 (Utilities|SpawnMesh (Math|Transform|MakeTransform _outlocation _outrotator (Variables|Pillar|Mid|GetPillarScale)) (Variables|StaticMesh|GetPillarMesh)))
        (return _meshcompref_2))
      (:Upper
        (bind _meshcompref_3 (Utilities|SpawnMesh (Math|Transform|MakeTransform _outlocation_2 _outrotator_2 (Variables|Pillar|Upper|GetPillarScaleUpper)) (Variables|StaticMesh|GetUpperPillarMesh)))
        (return _meshcompref_3)))
    (else
      ;[1 1 1] wall
      (Utilities|PositionOfMesh CounterIndex
        (:Lower
          (bind _meshcompref_4 (Utilities|SpawnMesh Transform (Variables|StaticMesh|GetLowerWallMesh)))
          (return _meshcompref_4))
        (:Mid
          (bind _meshcompref_5 (Utilities|SpawnMesh Transform (Variables|StaticMesh|GetWallMesh)))
          (return _meshcompref_5))
        (:Upper
          (bind _meshcompref_6 (Utilities|SpawnMesh Transform (Variables|StaticMesh|GetUpperWallMesh)))
          (return _meshcompref_6))))))